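; Character inventory Blueprint that tracks the items held in an Items collection.
; It exposes functions to add, check for and remove an item.
; Adding an item also prints a pickup message built from the item and "Picked Up".
; The event graph holds no active logic, so all behavior runs through these function calls.
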(fn `Add Item`
  (params (Item :type String))
  (`KismetArrayLibrary.Array_Add` (`self.Items`) Item)
  (`KismetSystemLibrary.PrintString` (`KismetStringLibrary.Concat_StrStr` Item " Picked Up")))

(fn `Has Item`
  (params (Item :type String))
  (returns (bHasItem :type Boolean))
  (return (`KismetArrayLibrary.Array_Contains` (`self.Items`) Item)))

(fn `Remove Item`
  (params (Item :type String))
  (`KismetArrayLibrary.Array_RemoveItem` (`self.Items`) Item))