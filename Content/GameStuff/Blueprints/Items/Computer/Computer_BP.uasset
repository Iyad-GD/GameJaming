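; Interactable computer actor that opens and closes a full computer screen UI when the player interacts with it.
; A FlipFlop on Interact alternates between pausing the game with a new CompScreen_WBP, visible cursor and Game and UI input, and unpausing with game-only input.
; Closing removes all widgets rather than just the computer screen, and the Triggered flag set on opening is never reset here.
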(event `/Game/GameStuff/Blueprints/GameMode/Interaction.Interact`
  (params (`Interacting Actor` :type "Actor Object Reference"))
  (bind _returnvalue (`GameplayStatics.GetPlayerController` 0))
  (bind _returnvalue_2 (`GameplayStatics.GetPlayerController` 0))
  (`/Engine/EditorBlueprintResources/StandardMacros.FlipFlop`
    (:`A`
      (`GameplayStatics.SetGamePaused` true)
      (bind _returnvalue_3 (`|CreateWidget` "/Game/GameStuff/Blueprints/Items/Computer/CompScreen_WBP.CompScreen_WBP_C"))
      (`UserWidget.AddToViewport` _returnvalue_3 0)
      (set `self.Triggered` true)
      (set `PlayerController.bShowMouseCursor` true _returnvalue)
      (`WidgetBlueprintLibrary.SetInputMode_GameAndUIEx` _returnvalue null))
    (:`B`
      (`GameplayStatics.SetGamePaused` false)
      (`WidgetLayoutLibrary.RemoveAllWidgets`)
      (set `PlayerController.bShowMouseCursor` false _returnvalue_2)
      (`WidgetBlueprintLibrary.SetInputMode_GameOnly` _returnvalue_2))))

(fn `UserConstructionScript`)