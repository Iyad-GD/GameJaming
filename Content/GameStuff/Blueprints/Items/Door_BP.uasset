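; BP_Door is an interactable door that swings its static mesh between closed and open when a BP_FirstPersonCharacter interacts with it.
; A timeline drives a rotator lerp on the mesh, playing to open and reversing to close.
; Closing requires the door to be open and NeededItem in the character's inventory; every other interaction opens it, so opening needs no item.
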(event `/Game/GameStuff/Blueprints/GameMode/Interaction.Interact`
  (params (`Interacting Actor` :type "Actor Object Reference"))
  (bind _asbp_first_person_character (cast `/Game/GameStuff/Blueprints/Character/BP_FirstPersonCharacter` `Interacting Actor`))
  (if (and (`self.bIsOpen`) (`KismetArrayLibrary.Array_Contains` (`/Game/GameStuff/Blueprints/Character/BP_FirstPersonCharacter.Inventory` _asbp_first_person_character) (`self.NeededItem`)))
    (set `self.bIsOpen` false)
    (bind (_direction _newtrack_0) (`Timeline|Timeline` :!via `Reverse` :!label _label)
      (:`Update`
        (`SceneComponent.K2_SetRelativeRotation` (`self.StaticMesh`) (`KismetMathLibrary.RLerp` (struct) (`self.Lerp B`) _newtrack_0) false false)))
    (else
      (set `self.bIsOpen` true)
      (goto _label))))

(fn `UserConstructionScript`)