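; Item checker actor that tests whether the first-person player carries a required item when they enter its box.
; On Box overlap, it casts to BP_FirstPersonCharacter and queries the Inventory component for the RequıredItem.
; A match removes the item from the inventory and prints a removal message; otherwise it only prints a placeholder failure string.
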(event `self.ReceiveBeginPlay`)

(event `self.Box.OnComponentBeginOverlap`
  (params (OverlappedComponent :type "PrimitiveComponent Object Reference") (OtherActor :type "Actor Object Reference") (OtherComp :type "PrimitiveComponent Object Reference") (OtherBodyIndex :type Integer) (bFromSweep :type Boolean) (SweepResult :type "HitResult Structure (by ref)"))
  (bind `_requıred_item` (`self.Requıred Item`))
  (bind _asbp_first_person_character (cast `/Game/GameStuff/Blueprints/Character/BP_FirstPersonCharacter` OtherActor))
  (bind _bhasitem (`/Game/GameStuff/Blueprints/Character/Inventory.Has Item` (`self.GetComponentByClass` _asbp_first_person_character "/Game/GameStuff/Blueprints/Character/Inventory.Inventory_C") (`self.Requıred Item`)))
  (if _bhasitem
    (`/Game/GameStuff/Blueprints/Character/Inventory.Remove Item` (`/Game/GameStuff/Blueprints/Character/BP_FirstPersonCharacter.Inventory` _asbp_first_person_character) `_requıred_item`)
    (`KismetSystemLibrary.PrintString` (`KismetStringLibrary.Concat_StrStr` `_requıred_item` " Removed"))
    (else
      (`KismetSystemLibrary.PrintString` "YOU ARE NOT GAY"))))

(fn `UserConstructionScript`)