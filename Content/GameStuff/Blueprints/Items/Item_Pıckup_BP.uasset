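; Item pickup actor that adds its named item to the player's inventory when the player presses E nearby.
; A Box component's overlap events toggle a PlayerNear flag, with no actor type check at that point.
; Tick polls the E key while the flag is set, casts the overlapping actor to BP_FirstPersonCharacter, passes ItemName to its Inventory component's AddItem, then destroys the pickup.
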(event `self.ReceiveBeginPlay`
  (`self.EnableInput` (`GameplayStatics.GetPlayerController` 0)))

(event `self.ReceiveTick`
  (params (DeltaSeconds :type "Float (single-precision)"))
  (if (`self.PlayerNear?`)
    (if (`PlayerController.IsInputKeyDown` (`GameplayStatics.GetPlayerController` 0) "E")
      (bind _asbp_first_person_character (cast `/Game/GameStuff/Blueprints/Character/BP_FirstPersonCharacter` (stale `self.Box.OnComponentBeginOverlap` OtherActor)))
      (`/Game/GameStuff/Blueprints/Character/Inventory.Add Item` (`self.GetComponentByClass` _asbp_first_person_character "/Game/GameStuff/Blueprints/Character/Inventory.Inventory_C") (`self.Item Name`))
      (`self.K2_DestroyActor`))))

(event `self.Box.OnComponentBeginOverlap`
  (params (OverlappedComponent :type "PrimitiveComponent Object Reference") (OtherActor :type "Actor Object Reference") (OtherComp :type "PrimitiveComponent Object Reference") (OtherBodyIndex :type Integer) (bFromSweep :type Boolean) (SweepResult :type "HitResult Structure (by ref)"))
  (set `self.PlayerNear?` true))

(event `self.Box.OnComponentEndOverlap`
  (params (OverlappedComponent :type "PrimitiveComponent Object Reference") (OtherActor :type "Actor Object Reference") (OtherComp :type "PrimitiveComponent Object Reference") (OtherBodyIndex :type Integer))
  (set `self.PlayerNear?` false))

(fn `UserConstructionScript`)