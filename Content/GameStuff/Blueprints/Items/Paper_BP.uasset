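; Paper_BP is an interactable paper item that can be signed once the player carries the needed item, indicated as a pen.
; Interact casts the interacting actor to BP_FirstPersonCharacter and checks its Inventory for NeededItem.
; If the item is present, the static mesh swaps to the signed sheet.
; Otherwise it prints a hint and shows an updated objective image on the InGameUIWBP widget, found by class lookup.
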(event `/Game/GameStuff/Blueprints/GameMode/Interaction.Interact`
  (params (`Interacting Actor` :type "Actor Object Reference"))
  (bind _asbp_first_person_character (cast `/Game/GameStuff/Blueprints/Character/BP_FirstPersonCharacter` `Interacting Actor`))
  (if (`KismetArrayLibrary.Array_Contains` (`/Game/GameStuff/Blueprints/Character/BP_FirstPersonCharacter.Inventory` _asbp_first_person_character) (`self.Needed Item`))
    (`StaticMeshComponent.SetStaticMesh` (`self.StaticMesh`) "/Game/GameStuff/Blueprints/Key_and_Paper/PaperFull/FULLSHEETSIGNED/StaticMeshes/FULLSHEETSIGNED.FULLSHEETSIGNED")
    (else
      (`KismetSystemLibrary.PrintString` "You need a Pen")
      (bind _foundwidgets (`WidgetBlueprintLibrary.GetAllWidgetsOfClass` "/Game/GameStuff/Blueprints/UI/In-Game-UI-WBP.In-Game-UI-WBP_C"))
      (bind _objectiveimage (`/Game/GameStuff/Blueprints/UI/In-Game-UI-WBP.ObjectiveImage` (`|GetArrayItem` _foundwidgets)))
      (set `Widget.Visibility` "Visible" _objectiveimage)
      (`Image.SetBrushFromTexture` _objectiveimage "/Game/GameStuff/Images/Cutscenes/1_Sign_Paper/Obj1_5.Obj1_5" true))))

(fn `UserConstructionScript`)