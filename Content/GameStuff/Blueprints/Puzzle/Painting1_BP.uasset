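; Painting puzzle actor that stays hidden until the player holds a required item.
; The construction script applies the configurable Model to its static mesh.
; BeginPlay hides the mesh and caches the first-person player character.
; The PuzzlesAppear event makes the mesh visible only if that character's Inventory contains RequiredItem.
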(event `self.ReceiveBeginPlay`
  (`SceneComponent.SetVisibility` (`self.StaticMesh`) false false)
  (bind _asbp_first_person_character (cast `/Game/GameStuff/Blueprints/Character/BP_FirstPersonCharacter` (`GameplayStatics.GetPlayerCharacter` 0))))

(event `/Game/GameStuff/Blueprints/GameMode/Interaction.PuzzlesAppear`
  (if (`KismetArrayLibrary.Array_Contains` (`/Game/GameStuff/Blueprints/Character/BP_FirstPersonCharacter.Inventory` (stale `self.ReceiveBeginPlay` _asbp_first_person_character)) (`self.RequiredItem`))
    (`SceneComponent.SetVisibility` (`self.StaticMesh`) true false)))

(fn `UserConstructionScript`
  (`StaticMeshComponent.SetStaticMesh` (`self.StaticMesh`) (`self.Model`)))