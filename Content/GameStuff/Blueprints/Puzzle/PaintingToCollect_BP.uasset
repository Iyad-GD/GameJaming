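; A collectible painting actor for puzzles that puts an item into the first-person character's inventory.
; The construction script applies a configurable mesh, and BeginPlay caches the player character.
; When the PuzzlesCollect event fires, it adds RequiredItem to that inventory and destroys itself.
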(event `self.ReceiveBeginPlay`
  (bind _asbp_first_person_character (cast `/Game/GameStuff/Blueprints/Character/BP_FirstPersonCharacter` (`GameplayStatics.GetPlayerCharacter` 0))))

(event `/Game/GameStuff/Blueprints/GameMode/Interaction.PuzzlesCollect`
  (`KismetArrayLibrary.Array_Add` (`/Game/GameStuff/Blueprints/Character/BP_FirstPersonCharacter.Inventory` (stale `self.ReceiveBeginPlay` _asbp_first_person_character)) (`self.RequiredItem`))
  (`self.K2_DestroyActor`))

(fn `UserConstructionScript`
  (`StaticMeshComponent.SetStaticMesh` (`self.StaticMesh`) (`self.NewMesh`)))