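; Puzzle manager that tracks Painting1_BP actors and completes an objective once enough of them are visible.
; BeginPlay gathers the paintings, and Tick advances an index whenever the painting at that index has a visible mesh, checking them in array order.
; Each advance prints a debug fail until the index equals TargetIndex, then prints success and hides the InGameUIWBP objective image if its material matches Obj6.
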(event `self.ReceiveBeginPlay`
  (bind _outactors (`GameplayStatics.GetAllActorsOfClass` "/Game/GameStuff/Blueprints/Puzzle/Painting1_BP.Painting1_BP_C")))

(event `self.ReceiveTick`
  (params (DeltaSeconds :type "Float (single-precision)"))
  (if (`SceneComponent.IsVisible` (`/Game/GameStuff/Blueprints/Puzzle/Painting1_BP.StaticMesh` (`|GetArrayItem` (stale `self.ReceiveBeginPlay` _outactors) (`self.IndexLoop`))))
    (`/Engine/EditorBlueprintResources/StandardMacros.IncrementInt` (`self.IndexLoop`)
      (:`  `
        (`self.CustomEvent`)))))

(event `CustomEvent`
  (if (== (`self.IndexLoop`) (`self.TargetIndex`))
    (`KismetSystemLibrary.PrintString` "SUCCESSS")
    (bind _foundwidgets (`WidgetBlueprintLibrary.GetAllWidgetsOfClass` "/Game/GameStuff/Blueprints/UI/In-Game-UI-WBP.In-Game-UI-WBP_C"))
    (bind _objectiveimage (`/Game/GameStuff/Blueprints/UI/In-Game-UI-WBP.ObjectiveImage` (`|GetArrayItem` _foundwidgets)))
    (bind _returnvalue (`Image.GetDynamicMaterial` _objectiveimage))
    (if (== _returnvalue "/Game/GameStuff/Images/Cutscenes/6_On_The_Walls/Obj6.Obj6")
      (set `Widget.Visibility` "Hidden" _objectiveimage))
    (else
      (`KismetSystemLibrary.PrintString` "FAIIL"))))

(fn `UserConstructionScript`)